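; BP_VisibleObject is the visible mesh of an item, attached to a parent actor, that doubles as a melee weapon hitbox.
; It applies ObjectMesh on BeginPlay, and attack events toggle its overlap collision, resetting the ignore list to the parent on activation.
; Overlapping a non-ignored actor with Component_Parameters lowers a parameter by the weapon class's default value and reports a "Hit" damage event to AI perception.
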(event OnComponentBeginOverlap(Object)
  (params (OverlappedComponent :type Primitive%20Component%20Object%20Reference) (OtherActor :type Actor%20Object%20Reference) (OtherComp :type Primitive%20Component%20Object%20Reference) (OtherBodyIndex :type Integer) (bFromSweep :type Boolean) (SweepResult :type Hit%20Result%20Structure%20%28by%20ref%29))
  (bind _returnvalue (Actor|GetComponentbyClass OtherActor "/Game/Main/Components/Component_Parameters.Component_Parameters_C"))
  (if (not (Utilities|Array|ContainsItem (Variables|Default|GetIgnored%20Actors) OtherActor))
    (Utilities|IsValid _returnvalue
      (:Is%20Valid
        (bind _asbpc_item_weapon_base (Utilities|Casting|CastToBPC_Item_Weapon_BaseClass (Variables|Default|GetItem)))
        (Default|ChangeParameter _returnvalue "NewEnumerator0" (- 0.0 (Utilities|GetClassDefaults _asbpc_item_weapon_base)))
        (Class|AISenseDamage|ReportDamageEvent OtherActor (Actor|GetParentActor) (Utilities|GetClassDefaults _asbpc_item_weapon_base) (Transformation|GetWorldLocation (Variables|Default|GetObject)) "0, 0, 0" "Hit")))))

(event Custom|Set%20Attack%20Inactive
  (Collision|SetCollisionProfileName (Variables|Default|GetObject) "NoCollision" true :!class /Script/Engine.PrimitiveComponent))

(event Custom|Set%20Attack%20Active
  (Utilities|Array|Clear (Variables|Default|GetIgnored%20Actors))
  (Utilities|Array|Add (Variables|Default|GetIgnored%20Actors) (Variables|Default|GetParent%20Actor))
  (Collision|SetCollisionProfileName (Variables|Default|GetObject) "OverlapAll" true :!class /Script/Engine.PrimitiveComponent))

(event EventBeginPlay
  (Components|StaticMesh|SetStaticMesh (Variables|Default|GetObject) (Variables|Default|GetObject%20Mesh)))

(event Collision|EventActorBeginOverlap
  (params (OtherActor :type Actor%20Object%20Reference)))

(event EventTick
  (params (DeltaSeconds :type Float%20%28single-precision%29)))

(fn ConstructionScript)