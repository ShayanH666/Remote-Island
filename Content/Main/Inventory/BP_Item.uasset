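; World pickup actor for an inventory item, taking its mesh and "Pick up" prompt name from the Item class defaults.
; BeginPlay applies optional physics with an unwalkable slope, finds BP_SceneManager and destroys the actor if already picked up.
; PickUp adds one item to the given inventory and, on success, flags its PlacedItems entry, matched by display name, then destroys itself.
; SpawnSound pairs audio with an AI noise event.
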(event Custom|Pick%20Up
  (params (Inventory :type Component%20Inventory%20Object%20Reference))
  (bind _success (Default|AddItem Inventory (Variables|Default|GetItem) 1))
  (if _success
    (CallFunction|ChangeSceneManagerReference)
    (Actor|DestroyActor)))

(event EventBeginPlay
  (bind _physics_simulation (Variables|Default|GetPhysics%20Simulation))
  (Utilities|FlowControl|Sequence
    (:then_0
      (Physics|SetSimulatePhysics (Variables|Default|GetStaticMesh) _physics_simulation)
      (if _physics_simulation
        (Class|PrimitiveComponent|SetWalkableSlopeOverride (Variables|Default|GetStaticMesh) (Utilities|Struct|MakeWalkableSlopeOverride "WalkableSlope_Unwalkable" 0.0))))
    (:then_1
      (bind _outactors (Actor|GetAllActorsOfClass "/Game/Main/Blueprints/Essential/BP_SceneManager.BP_SceneManager_C"))
      (Variables|Default|SetScene%20Manager (Utilities|Array|Get(acopy) _outactors)))
    (:then_2
      (if (CallFunction|AlreadyPickedUp)
        (Actor|DestroyActor)))))

(event Collision|EventActorBeginOverlap
  (params (OtherActor :type Actor%20Object%20Reference)))

(event EventTick
  (params (DeltaSeconds :type Float%20%28single-precision%29)))

(fn ConstructionScript
  (Components|StaticMesh|SetStaticMesh (Variables|Default|GetStaticMesh) (.Mesh (Utilities|GetClassDefaults (Variables|Default|GetItem)))))

(fn SpawnSound
  (params (Sound :type Sound%20Base%20Object%20Reference) (Loudness :type Float%20%28double-precision%29) (MaxRange :type Float%20%28double-precision%29) (Tag :type Name))
  (bind _staticmesh (Variables|Default|GetStaticMesh))
  (bind _returnvalue (Transformation|GetWorldLocation _staticmesh))
  (Audio|SpawnSoundatLocation Sound _returnvalue "0, 0, 0" Loudness 1.0 0.0 0 0)
  (Class|AISenseHearing|ReportNoiseEvent _returnvalue Loudness self MaxRange Tag))

(fn ChangeSceneManagerReference
  (bind _self self)
  (bind _returnvalue (Utilities|GetDisplayName _self))
  (for (_array_element _array_index) (Variables|/Game/Main/Blueprints/Essential/BP_SceneManager.BP_SceneManager_C|GetPlaced%20Items (Variables|Default|GetScene%20Manager))
    (if (Utilities|Enum|Equal(Enum) (.actorname _array_element) _returnvalue)
      (Utilities|Array|SetArrayElem (Variables|/Game/Main/Blueprints/Essential/BP_SceneManager.BP_SceneManager_C|GetPlaced%20Items (Variables|Default|GetScene%20Manager)) _array_index (Utilities|Struct|MakeF_PlacedItem _returnvalue true))
      (return))))

(fn AlreadyPickedUp
  (for _array_element (Variables|/Game/Main/Blueprints/Essential/BP_SceneManager.BP_SceneManager_C|GetPlaced%20Items (Variables|Default|GetScene%20Manager))
    (if (Utilities|Enum|Equal(Enum) (.actorname _array_element) (Utilities|GetDisplayName self))
      (return (.pickedup _array_element)))))

(fn GetActionWidgetText
  (return (Utilities|String|Append "Pick up " (Utilities|String|ToString(Text) (.Name (Utilities|GetClassDefaults (Variables|Default|GetItem)))))))