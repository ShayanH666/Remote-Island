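; Box trigger that switches the set of streamed levels when the player character enters it.
; On overlap it unloads levels tracked in Main_GameInstance that are absent from its LevelsToStream, removing them from that list during the loop.
; It loads its own levels asynchronously, staggered through a delayed DoN loop that later resets, and records each in the GameInstance.
; It also passes the set to BP_SceneManager, found at construction, for saving.
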(event OnComponentBeginOverlap(Box)
  (params (OverlappedComponent :type Primitive%20Component%20Object%20Reference) (OtherActor :type Actor%20Object%20Reference) (OtherComp :type Primitive%20Component%20Object%20Reference) (OtherBodyIndex :type Integer) (bFromSweep :type Boolean) (SweepResult :type Hit%20Result%20Structure%20%28by%20ref%29))
  (if (== OtherActor (Game|GetPlayerCharacter 0))
    (Utilities|FlowControl|Sequence
      (:then_0
        (for _array_element (Variables|/Game/Main/Libraries/Main_GameInstance.Main_GameInstance_C|GetStreamed%20Levels (Variables|Default|GetAs%20Main%20Game%20Instance))
          (if (not (Utilities|Array|ContainsItem (Variables|Default|GetLevels%20to%20Stream) _array_element))
            (Class|GameplayStatics|UnloadStreamLevelbySoftObjectPtr _array_element false)
            (Utilities|Array|RemoveItem (Variables|/Game/Main/Libraries/Main_GameInstance.Main_GameInstance_C|GetStreamed%20Levels (Variables|Default|GetAs%20Main%20Game%20Instance)) _array_element))))
      (:then_1
        (bind _counter (Utilities|FlowControl|DoN (Utilities|Array|Length (Variables|Default|GetLevels%20to%20Stream)) :!label _label)
          (:Exit
            (CallFunction|LoadLevel (Utilities|Array|Get(acopy) (Variables|Default|GetLevels%20to%20Stream) (- _counter 1)))
            (Utilities|FlowControl|Delay 0.02)
            (goto _label))))
      (:then_2
        (Utilities|FlowControl|Delay (* (Utilities|Array|Length (Variables|Default|GetLevels%20to%20Stream)) 0.05))
        (goto _label Reset))
      (:then_3
        (Default|SaveStreamedLevels (Variables|Default|GetScene%20Manager) (Variables|Default|GetLevels%20to%20Stream))))))

(event Custom|Load%20Level
  (params (Level :type World%20Soft%20Object%20Reference))
  (Class|GameplayStatics|LoadStreamLevelbySoftObjectPtr Level true false)
  (Utilities|Array|AddUnique (Variables|/Game/Main/Libraries/Main_GameInstance.Main_GameInstance_C|GetStreamed%20Levels (Variables|Default|GetAs%20Main%20Game%20Instance)) Level))

(event EventBeginPlay
  (bind _asmain_game_instance (Utilities|Casting|CastToMain_GameInstance (Game|GetGameInstance)))
  (Variables|Default|SetAs%20Main%20Game%20Instance _asmain_game_instance))

(event Collision|EventActorBeginOverlap
  (params (OtherActor :type Actor%20Object%20Reference)))

(event EventTick
  (params (DeltaSeconds :type Float%20%28single-precision%29)))

(fn ConstructionScript
  (bind _outactors (Actor|GetAllActorsOfClass "/Game/Main/Blueprints/Essential/BP_SceneManager.BP_SceneManager_C"))
  (Variables|Default|SetScene%20Manager (Utilities|Array|Get(acopy) _outactors)))