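; Skydome actor that sets up sun and sky lighting for its Hours time of day once at BeginPlay.
; It pitches the directional light from Hours, samples SunColor and SkyColor curves for light color and alpha-driven intensity, then updates sun direction, brightness and the sky material.
; Tick is empty; the logic that would advance and wrap Hours over 24 is disconnected, so this graph does not animate time.
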(event EventBeginPlay
  (bind _skylight (Variables|Default|GetSkyLight))
  (bind _sky_color (Variables|Default|GetSky%20Color))
  (bind _hours (Variables|Default|GetHours))
  (bind _directional_light_actor (Variables|Default|GetDirectional%20light%20actor))
  (bind _sun_color (Variables|Default|GetSun%20Color))
  (bind _hours_2 (Variables|Default|GetHours))
  (bind _returnvalue (Math|Curves|GetLinearColorValue _sky_color _hours_2))
  (bind _returnvalue_2 (Math|Curves|GetLinearColorValue _sun_color _hours))
  (bind _lightcomponent (Variables|/Script/Engine.Light|GetLightComponent _directional_light_actor))
  (bind _a (Math|Color|BreakColor _returnvalue_2))
  (Transformation|SetActorRotation (Variables|Default|GetDirectional%20light%20actor) (Math|Rotator|MakeRotator 0.0 (+ (* (Variables|Default|GetHours) 15.0) 9e+01) 0.0))
  (CallFunction|UpdateSunDirection)
  (Rendering|Components|Light|SetLightColor _lightcomponent _returnvalue_2 true)
  (Rendering|Components|Light|SetIntensity _lightcomponent (* _a 2.5))
  (Variables|Default|SetSun%20brightness (* _a 1e+02))
  (Rendering|Components|Light|SetLightColor _skylight _returnvalue)
  (Rendering|Components|Light|SetIntensity _skylight (.A (Math|Color|BreakColor _returnvalue)))
  (CallFunction|RefreshMaterial))

(event Collision|EventActorBeginOverlap
  (params (OtherActor :type Actor%20Object%20Reference)))

(event EventTick
  (params (DeltaSeconds :type Float%20%28single-precision%29)))

(fn ConstructionScript
  (|CallParentFunction))