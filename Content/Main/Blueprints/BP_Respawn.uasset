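; BP_Respawn is an interactable save point that sets the checkpoint and opens the level-up screen.
; Interact turns on its Niagara effect, has the BP_SceneManager found at BeginPlay respawn enemies, and stores its transform as that manager's checkpoint.
; It then shows WB_LevelUp with UI-only input and a visible cursor.
; GetActionWidgetText supplies the "Activate Save Point" prompt.
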(event EventBeginPlay
  (bind _outactors (Actor|GetAllActorsOfClass "/Game/Main/Blueprints/Essential/BP_SceneManager.BP_SceneManager_C"))
  (Variables|Default|SetScene%20Manager (Utilities|Array|Get(acopy) _outactors)))

(event Collision|EventActorBeginOverlap
  (params (OtherActor :type Actor%20Object%20Reference)))

(event EventTick
  (params (DeltaSeconds :type Float%20%28single-precision%29)))

(event EventInteract
  (bind _returnvalue (Game|GetPlayerController 0))
  (bind _scene_manager (Variables|Default|GetScene%20Manager))
  (Components|Activation|Activate (Variables|Default|GetNiagara) false)
  (Default|RespawnEnemies _scene_manager)
  (Variables|/Game/Main/Blueprints/Essential/BP_SceneManager.BP_SceneManager_C|SetCheckpoint _scene_manager (Transformation|GetActorTransform))
  (bind _returnvalue_2 (UserInterface|CreateWidget "/Game/Main/Widgets/WB_LevelUp.WB_LevelUp_C" _returnvalue))
  (UserInterface|Viewport|AddtoViewport _returnvalue_2 0)
  (Input|SetInputModeUIOnly _returnvalue _returnvalue_2 "DoNotLock")
  (Variables|/Script/Engine.PlayerController|SetbShowMouseCursor _returnvalue true))

(fn ConstructionScript)

(fn GetActionWidgetText
  (return "Activate Save Point"))