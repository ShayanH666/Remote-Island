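; BP_Tornado is a moving tornado that lifts Characters and BP_Items caught in its capsule.
; Each tick it polls capsule overlaps to fill AffectedActors, which end-overlap events prune, and sweeps them upward, moving an item's mesh rather than the actor.
; It snaps to a WorldStatic trace along its Arrow with random drift biased toward +Y, destroying itself when the impact point is zero.
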(event OnComponentEndOverlap(Capsule)
  (params (OverlappedComponent :type Primitive%20Component%20Object%20Reference) (OtherActor :type Actor%20Object%20Reference) (OtherComp :type Primitive%20Component%20Object%20Reference) (OtherBodyIndex :type Integer))
  (Utilities|Array|RemoveItem (Variables|Default|GetAffected%20Actors) OtherActor))

(event EventBeginPlay)

(event Collision|EventActorBeginOverlap
  (params (OtherActor :type Actor%20Object%20Reference)))

(event EventTick
  (params (DeltaSeconds :type Float%20%28single-precision%29))
  (bind _returnvalue (Utilities|Time|GetWorldDeltaSeconds))
  (bind _returnvalue_2 (Utilities|Time|GetWorldDeltaSeconds))
  (bind _arrow (Variables|Default|GetArrow))
  (bind _capsule (Variables|Default|GetCapsule))
  (bind _returnvalue_3 (Transformation|GetWorldLocation _arrow))
  (bind _returnvalue_4 (* _returnvalue_2 3e+03))
  (Utilities|FlowControl|Sequence
    (:then_0
      (for _array_element (Variables|Default|GetAffected%20Actors)
        (bind _asbp_item (Utilities|Casting|CastToBP_Item _array_element)
          (:then
            (Transformation|AddWorldOffset (Variables|/Game/Main/Inventory/BP_Item.BP_Item_C|GetStaticMesh _asbp_item) (Math|Vector|MakeVector 0.0 0.0 _returnvalue_4) true false))
          (:CastFailed
            (Transformation|AddActorWorldOffset _array_element (Math|Vector|MakeVector 0.0 0.0 _returnvalue_4) true)))))
    (:then_1
      (bind _outhit (Collision|LineTraceForObjects _returnvalue_3 (+ _returnvalue_3 (* (Math|Vector|GetForwardVector _arrow) 2e+04)) (Utilities|Array|MakeArray "ObjectTypeQuery1") false 0 "None"))
      (if (Math|Vector|Equal(Vector) (.ImpactPoint (Collision|BreakHitResult _outhit)) "0, 0, 0" 0.0)
        (Actor|DestroyActor)
        (else
          (Transformation|SetActorLocation (+ (.ImpactPoint (Collision|BreakHitResult _outhit)) (Math|Vector|MakeVector (Math|Random|RandomFloatinRange (* _returnvalue -1e+02) (* _returnvalue 1e+02)) (Math|Random|RandomFloatinRange (* _returnvalue 2e+02) (* _returnvalue 3e+02)) 0.0)) true false))))
    (:then_2
      (Utilities|IsValid _capsule
        (:Is%20Valid
          (bind _outactors (Collision|ComponentOverlapActors _capsule (Transformation|GetWorldTransform _capsule) (Utilities|Array|MakeArray "ObjectTypeQuery1" "ObjectTypeQuery2" "ObjectTypeQuery3" "ObjectTypeQuery4") 0))
          (for _array_element_2 _outactors
            (bind _ascharacter (Utilities|Casting|CastToCharacter _array_element_2)
              (:then
                (Utilities|Array|AddUnique (Variables|Default|GetAffected%20Actors) _ascharacter))
              (:CastFailed
                (bind _asbp_item_2 (Utilities|Casting|CastToBP_Item _array_element_2))
                (Utilities|Array|AddUnique (Variables|Default|GetAffected%20Actors) _asbp_item_2)))))))))

(fn ConstructionScript)