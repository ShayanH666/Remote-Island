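; BP_NPC is an enemy character with a montage-driven melee attack, a weapon held as a child actor, and a kill state tracked by the scene manager.
; On BeginPlay it finds BP_SceneManager and destroys itself if its PlacedEnemies entry, matched by display name, is marked killed.
; Death runs once, destroying the controller, ragdolling the mesh, awarding player XP and marking that entry killed.
; GetDamage returns zero here.
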(event EventBeginPlay
  (bind _outactors (Actor|GetAllActorsOfClass "/Game/Main/Blueprints/Essential/BP_SceneManager.BP_SceneManager_C"))
  (Variables|Default|SetScene%20Manager (Utilities|Array|Get(acopy) _outactors))
  (if (CallFunction|AlreadyKilled)
    (Actor|DestroyActor)))

(event Collision|EventActorBeginOverlap
  (params (OtherActor :type Actor%20Object%20Reference)))

(event EventTick
  (params (DeltaSeconds :type Float%20%28single-precision%29)))

(event EventMeeleAttack
  (Animation|Montage|PlayMontage (Variables|Character|GetMesh) "/Game/Main/AI/NPC/Animations/Attack_PrimaryA_Montage.Attack_PrimaryA_Montage"))

(event EventDeath
  (bind _returnvalue (Pawn|GetController))
  (bind _mesh (Variables|Character|GetMesh))
  (Utilities|FlowControl|DoOnce false
    (:Completed
      (Utilities|IsValid _returnvalue
        (:Is%20Valid
          (Actor|DestroyActor _returnvalue))
        (:Is%20Not%20Valid
          _))
      (Collision|SetCollisionProfileName _mesh "Ragdoll" true :!class /Script/Engine.PrimitiveComponent)
      (Physics|SetSimulatePhysics _mesh true)
      (Default|AddXP (Actor|GetComponentbyClass (Game|GetPlayerCharacter 0) "/Game/Main/Components/Component_Level.Component_Level_C") 500)
      (CallFunction|ChangeSceneManagerReference))))

(fn ConstructionScript)

(fn ChangeSceneManagerReference
  (bind _self self)
  (bind _returnvalue (Utilities|GetDisplayName _self))
  (for (_array_element _array_index) (Variables|/Game/Main/Blueprints/Essential/BP_SceneManager.BP_SceneManager_C|GetPlaced%20Enemies (Variables|Default|GetScene%20Manager))
    (if (Utilities|Enum|Equal(Enum) (.actorname _array_element) _returnvalue)
      (Utilities|Array|SetArrayElem (Variables|/Game/Main/Blueprints/Essential/BP_SceneManager.BP_SceneManager_C|GetPlaced%20Enemies (Variables|Default|GetScene%20Manager)) _array_index (Utilities|Struct|MakeF_PlacedEnemies _returnvalue true (.respawns _array_element))))))

(fn AlreadyKilled
  (for _array_element (Variables|/Game/Main/Blueprints/Essential/BP_SceneManager.BP_SceneManager_C|GetPlaced%20Enemies (Variables|Default|GetScene%20Manager))
    (if (Utilities|Enum|Equal(Enum) (.actorname _array_element) (Utilities|GetDisplayName self))
      (return (.killed _array_element)))))

(fn GetDamage
  (return 0.0))

(fn GetWeaponComponent
  (bind _asbp_visible_object (Utilities|Casting|CastToBP_VisibleObject (Variables|/Script/Engine.ChildActorComponent|GetChildActor (Variables|Default|GetBP_VisibleObject))))
  (return _asbp_visible_object))